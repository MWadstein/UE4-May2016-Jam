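; VR game mode that handles checkpoints, player death and respawn, and the game's ending.
; It stores the current checkpoint level and teleports the pawn to the RespawnPoint tagged with that level, behind camera fades.
; On death it also sends a reset to that level's enemy class and destroys all projectiles.
; The ending plays a sound, fades out, flags voiceovers as played on the game instance and reloads PersistentMap.
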(event `/Game/Blueprints/Interfaces/BPI_VRGameMode.SetCheckpoint`
  (params (Level :type Integer))
  ;[1 1 1] Set our new Checkpoint Level
  (set `self.CurrentPlayerLevel` Level))

(event `/Game/Blueprints/Interfaces/BPI_VRGameMode.SpawnPlayer`
  (params (Level :type Integer))
  ;[1 1 1] Debug Event - Testing
  (set `self.CurrentPlayerLevel` Level)
  (`self.RespawnPlayer`))

(event `self.ReceiveBeginPlay`
  ;[1 1 1] Begin Play
  (`PlayerCameraManager.SetManualCameraFade` :`self` (`GameplayStatics.GetPlayerCameraManager` 0) :`InFadeAmount` 1.0)
  (`KismetSystemLibrary.Delay` 2.0)
  (`self.RespawnPlayer`)
  (`PlayerCameraManager.StartCameraFade` :`self` (`GameplayStatics.GetPlayerCameraManager` 0) :`FromAlpha` 1.0 :`Duration` 3.0))

(event `RespawnPlayer`
  ;[1 1 1] Respawn Player at Current Checkpoint
  (bind _location (`self.GetSpawnPointLocation`))
  (`self.K2_SetActorLocationAndRotation` (`GameplayStatics.GetPlayerPawn` 0) (.location _location) (.rotation _location) false false))

(event `/Game/Blueprints/Interfaces/BPI_VRGameMode.HandlePlayerDied`
  ;[1 1 1] Handle Player Dieing
  (`self.ResetCurrentLevelEnemies`)
  (`self.RespawnPlayer`)
  (`PlayerCameraManager.StartCameraFade` :`self` (`GameplayStatics.GetPlayerCameraManager` 0) :`FromAlpha` 1.0 :`Duration` 3.0))

(event `/Game/Blueprints/Interfaces/BPI_VRGameMode.TriggerEndGame`
  ;[1 1 1] Handle the end of the game being triggered
  (`GameplayStatics.PlaySound2D` "/Game/Audio/17.17")
  (`KismetSystemLibrary.Delay` 28.0)
  (`PlayerCameraManager.StartCameraFade` :`self` (`GameplayStatics.GetPlayerCameraManager` 0) :`ToAlpha` 1.0 :`Duration` 4.0 :`bHoldWhenFinished` true)
  (`KismetSystemLibrary.Delay` 4.0)
  (set `/Game/Blueprints/Game/VRGameInstance.VoiceoversPlayed` true (cast `/Game/Blueprints/Game/VRGameInstance` (`GameplayStatics.GetGameInstance`) :!pure true))
  (`GameplayStatics.OpenLevel` "PersistentMap"))

(fn `GetSpawnPointLocation`
  (returns (Location :type "Transform Structure"))
  (bind _outactors (`GameplayStatics.GetAllActorsOfClass` "/Game/Blueprints/Helpers/RespawnPoint.RespawnPoint_C"))
  (for _array_element _outactors
    (if (== (`/Game/Blueprints/Helpers/RespawnPoint.Level` _array_element) (`self.CurrentPlayerLevel`))
      (break)))
  (return (`self.GetTransform` _array_element)))

(fn `ResetCurrentLevelEnemies`
  (bind _outactors (`GameplayStatics.GetAllActorsOfClass` (select `int` (`self.CurrentPlayerLevel`) :`0` null :`1` null :`2` "/Game/Blueprints/Enemies/Enemy_Level2.Enemy_Level2_C" :`3` "/Game/Blueprints/Enemies/Enemy_Level3.Enemy_Level3_C" :`4` "/Game/Blueprints/Enemies/Enemy_Level4.Enemy_Level4_C" :!type "Actor Class Reference")))
  (for _array_element _outactors
    (message `/Game/Blueprints/Interfaces/BPI_Enemy.HandleBeingReset` _array_element))
  (bind _outactors_2 (`GameplayStatics.GetAllActorsOfClass` "/Game/Blueprints/Enemies/Projectile.Projectile_C"))
  (for _array_element_2 _outactors_2
    (`self.K2_DestroyActor` _array_element_2))
  (return))

(fn `UserConstructionScript`)