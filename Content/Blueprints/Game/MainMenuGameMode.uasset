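; Game mode for the main menu, which fades the camera in from black on BeginPlay.
; It also carries level helpers keyed on CurrentPlayerLevel: one returns the transform of the matching RespawnPoint.
; The other sends a reset message to that level's enemy class, set only for levels 2 to 4, and destroys all projectiles.
; Neither helper is called within this graph.
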(event `self.ReceiveBeginPlay`
  (`PlayerCameraManager.StartCameraFade` :`self` (`GameplayStatics.GetPlayerCameraManager` 0) :`FromAlpha` 1.0 :`Duration` 3.0))

(fn `GetSpawnPointLocation`
  (returns (Location :type "Transform Structure"))
  (bind _outactors (`GameplayStatics.GetAllActorsOfClass` "/Game/Blueprints/Helpers/RespawnPoint.RespawnPoint_C"))
  (for _array_element _outactors
    (if (== (`/Game/Blueprints/Helpers/RespawnPoint.Level` _array_element) (`self.CurrentPlayerLevel`))
      (break)))
  (return (`self.GetTransform` _array_element)))

(fn `ResetCurrentLevelEnemies`
  (bind _outactors (`GameplayStatics.GetAllActorsOfClass` (select `int` (`self.CurrentPlayerLevel`) :`0` null :`1` null :`2` "/Game/Blueprints/Enemies/Enemy_Level2.Enemy_Level2_C" :`3` "/Game/Blueprints/Enemies/Enemy_Level3.Enemy_Level3_C" :`4` "/Game/Blueprints/Enemies/Enemy_Level4.Enemy_Level4_C" :!type "Actor Class Reference")))
  (for _array_element _outactors
    (message `/Game/Blueprints/Interfaces/BPI_Enemy.HandleBeingReset` _array_element))
  (bind _outactors_2 (`GameplayStatics.GetAllActorsOfClass` "/Game/Blueprints/Enemies/Projectile.Projectile_C"))
  (for _array_element_2 _outactors_2
    (`self.K2_DestroyActor` _array_element_2))
  (return))

(fn `UserConstructionScript`)