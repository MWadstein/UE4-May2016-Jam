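; Base turret-style enemy that faces the player every tick and fires projectiles, optionally starting invisible.
; Entering its detection sphere reveals it after a delay and starts a self-rescheduling timer that fires only on clear line-of-sight traces.
; Hits spawn an explosion and disable rather than destroy it, so a reset can restore it.
; The overlap check in IsPlayerStillNearUs, meant to gate refiring, is left unwired.
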(event `self.ReceiveBeginPlay`
  ;[1 1 1] Begin Play
  (`SceneComponent.SetVisibility` (`self.Root`) (not (`self.StartInvisible`)) true))

(event `self.ReceiveTick`
  (params (DeltaSeconds :type "Float (single-precision)"))
  (if (`self.IsDestroyed`)
    (`SceneComponent.SetVisibility` (`self.Root`) false true)
    (`self.SetActorTickEnabled` false)
    (else
      ;[1 1 1] Tick and face player
      (bind _location (message `/Game/Blueprints/Interfaces/BPI_Player.GetPlayerBodyLocation` (`GameplayStatics.GetPlayerPawn` 0)))
      (`self.SetActorRotation` (`KismetMathLibrary.FindLookAtRotation` (`self.K2_GetActorLocation`) _location)))))

(event `/Game/Blueprints/Interfaces/BPI_Enemy.HandleBeingHit`
  ;[1 1 1] Handle Being Hit
  (`GameplayStatics.SpawnEmitterAtLocation` "/Game/Particles/Part_EnemyExplosion.Part_EnemyExplosion" (`SceneComponent.K2_GetComponentLocation` (`self.Sphere`)))
  (`self.DisableEnemy`))

(event `FireAtPlayer`
  (bind (_returnvalue_location _returnvalue_rotation) (`KismetMathLibrary.BreakTransform` (`SceneComponent.K2_GetComponentToWorld` (`self.FiringPoint`))))
  ;[1 1 1] Fire at the Player Event
  (`KismetSystemLibrary.Delay` (`self.FiringDelay`))
  (if (`self.IsPlayerStillNearUs`)
    (`self.LOS To Player?`
      (:`LOS`
        (`|SpawnActorFromClass` "/Game/Blueprints/Enemies/Projectile.Projectile_C" (`KismetMathLibrary.MakeTransform` _returnvalue_location _returnvalue_rotation (0.1 0.1 0.1)) "Undefined" "OverrideRootScale" null (`self.ProjectileSpeed`)))
      (:`NO LOS`
        _))
    (bind _returnvalue (`KismetSystemLibrary.K2_SetTimer` null "FireAtPlayer" (`self.RefireDelay`)))
    (set `self.TimerHandle` _returnvalue)
    (else
      (`KismetSystemLibrary.K2_ClearTimerHandle` (`self.TimerHandle`)))))

(event `self.SphereCollision.OnComponentBeginOverlap`
  (params (OtherActor :type "Actor Object Reference") (OtherComp :type "PrimitiveComponent Object Reference") (OtherBodyIndex :type Integer) (bFromSweep :type Boolean) (SweepResult :type "HitResult Structure (by ref)"))
  ;[1 1 1] Overlap Player
  (`KismetSystemLibrary.Delay` (`self.DelayBeforeVisible`))
  (`SceneComponent.SetVisibility` (`self.Root`) true true)
  (`self.FireAtPlayer`))

(event `/Game/Blueprints/Interfaces/BPI_Enemy.HandleBeingReset`
  ;[1 1 1] Handle being reset to defaults
  (`self.ResetToDefaults`))

(fn `DisableEnemy`
  (`|ExecutionSequence`
    (:`then_0`
      (set `self.IsDestroyed` true))
    (:`then_1`
      (`PrimitiveComponent.SetCollisionEnabled` (`self.SphereCollision`) "NoCollision"))
    (:`then_2`
      (`PrimitiveComponent.SetCollisionEnabled` (`self.Sphere`) "NoCollision"))
    (:`then_3`
      (`KismetSystemLibrary.K2_ClearTimerHandle` (`self.TimerHandle`)))
    (:`then_4`
      (return))))

(fn `ResetToDefaults`
  (`|ExecutionSequence`
    (:`then_0`
      (`SceneComponent.SetVisibility` (`self.Root`) (not (`self.StartInvisible`)) true))
    (:`then_1`
      (`PrimitiveComponent.SetCollisionEnabled` (`self.SphereCollision`) "QueryOnly"))
    (:`then_2`
      (`PrimitiveComponent.SetCollisionEnabled` (`self.Sphere`) "QueryOnly"))
    (:`then_3`
      (`self.SetActorTickEnabled` true))
    (:`then_4`
      (set `self.IsDestroyed` false))
    (:`then_5`
      (return))))

(fn `UserConstructionScript`
  (`SphereComponent.SetSphereRadius` (`self.SphereCollision`) (`self.CollisionRadius`) true))