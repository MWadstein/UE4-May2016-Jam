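; VR player pawn that teleports between pads with the left motion controller and shoots with the right.
; A per-tick trace highlights targeted pads; the left trigger moves the player behind a camera fade and re-entry gate, or ends the game on broken pads.
; The right trigger traces to notify BPI_Enemy actors or spawn impact particles.
; Being hit fades to red and notifies the GameMode, which also receives debug-key spawn requests.
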(event `/Game/Blueprints/Interfaces/BPI_Player.HandleBeingHit`
  (if (not (`self.IsDieing`))
    ;[1 1 1] Handle us being hit event
    (set `self.IsDieing` true)
    (`PlayerCameraManager.StartCameraFade` (`GameplayStatics.GetPlayerCameraManager` 0) 0.0 1.0 1.0 (struct :`R` 1.0 :`A` 1.0) false false)
    (`KismetSystemLibrary.Delay` 1.1)
    (message `/Game/Blueprints/Interfaces/BPI_VRGameMode.HandlePlayerDied` (`GameplayStatics.GetGameMode`))
    (set `self.IsDieing` false)))

(event `self.ReceiveTick`
  (params (DeltaSeconds :type "Float (single-precision)"))
  (bind _teleportfiringpoint (`self.TeleportFiringPoint`))
  (bind _returnvalue (`SceneComponent.K2_GetComponentLocation` _teleportfiringpoint))
  ;[1 1 1] Our Laser Pointer each Tick
  (bind (_outhit _returnvalue_2) (`KismetSystemLibrary.LineTraceSingle` _returnvalue (+ _returnvalue (* (`KismetMathLibrary.GetForwardVector` (`SceneComponent.K2_GetComponentRotation` _teleportfiringpoint)) 1000.0)) "TraceTypeQuery3"))
  (if _returnvalue_2
    (set `self.HitActor` (`.HitActor` (`GameplayStatics.BreakHitResult` _outhit))) ; Save Pad Reference
  )
  (if (!= _returnvalue_2 (`self.TeleportPadTargetted`))
    (if (not (`self.TeleportPadTargetted`))
      (bind _output_get (set `self.TeleportPadTargetted` true))
      (message `/Game/Blueprints/Interfaces/BPI_TeleportLocation.ToggleColor` (`self.HitActor`) _output_get)
      (else
        (bind _output_get_2 (set `self.TeleportPadTargetted` false))
        (message `/Game/Blueprints/Interfaces/BPI_TeleportLocation.ToggleColor` (`self.HitActor`) _output_get_2)))))

(event `Key|MotionController_Left_Trigger`
  (params (Key :type "Key Structure" :default "AnyKey"))
  ;[1 1 1] Pull Left (Teleport) Trigger Event
  (:`Pressed`
    (if (not (`self.IsDieing`))
      (if (`self.TeleportPadTargetted`)
        (`/Engine/EditorBlueprintResources/StandardMacros.Gate` false :!label _label
          (:`Exit`
            (`self.CloseTeleportGate`)
            (`PlayerCameraManager.StartCameraFade` :`self` (`GameplayStatics.GetPlayerCameraManager` 0) :`FromAlpha` 0.0 :`ToAlpha` 1.0 :`Duration` 0.2 :`bHoldWhenFinished` true)
            (`KismetSystemLibrary.Delay` 0.2)
            (bind (_transform _isbroken) (message `/Game/Blueprints/Interfaces/BPI_TeleportLocation.GetTeleportLocation` (`self.HitActor`)))
            (if _isbroken
              (`PlayerCameraManager.StartCameraFade` :`self` (`GameplayStatics.GetPlayerCameraManager` 0) :`FromAlpha` 1.0 :`ToAlpha` 0.0 :`Duration` 0.2)
              (message `/Game/Blueprints/Interfaces/BPI_VRGameMode.TriggerEndGame` (`GameplayStatics.GetGameMode`))
              (else
                (`self.K2_SetActorLocationAndRotation` (.location _transform) (.rotation _transform))
                (`PlayerCameraManager.StartCameraFade` :`self` (`GameplayStatics.GetPlayerCameraManager` 0) :`FromAlpha` 1.0 :`ToAlpha` 0.0 :`Duration` 0.2)
                (`self.OpenTeleportGate`)))))))))

(event `OpenTeleportGate`
  ;[1 1 1] Pull Left (Teleport) Trigger Event
  (goto _label :!via `Open`))

(event `CloseTeleportGate`
  ;[1 1 1] Pull Left (Teleport) Trigger Event
  (goto _label :!via `Close`))

(event `Key|MotionController_Right_Trigger`
  (params (Key :type "Key Structure" :default "AnyKey"))
  (bind _gunfiringpoint (`self.GunFiringPoint`))
  (bind _returnvalue (`SceneComponent.K2_GetComponentLocation` _gunfiringpoint))
  ;[1 1 1] Pull Right (Gun) Trigger Event
  (:`Pressed`
    (bind (_outhit _returnvalue_2) (`KismetSystemLibrary.LineTraceSingle` :`Start` _returnvalue :`End` (+ _returnvalue (* (`KismetMathLibrary.GetForwardVector` (`SceneComponent.K2_GetComponentRotation` _gunfiringpoint)) 1000.0)) :`TraceChannel` "TraceTypeQuery4" :`DrawDebugType` "ForOneFrame"))
    (if _returnvalue_2
      (if (`KismetSystemLibrary.DoesImplementInterface` (`.HitActor` (`GameplayStatics.BreakHitResult` _outhit)) "/Game/Blueprints/Interfaces/BPI_Enemy.BPI_Enemy_C")
        (message `/Game/Blueprints/Interfaces/BPI_Enemy.HandleBeingHit` (`.HitActor` (`GameplayStatics.BreakHitResult` _outhit))) ; Tell the enemy it was hit
        (else
          (`GameplayStatics.SpawnEmitterAtLocation` "/Game/Particles/Part_GunHit.Part_GunHit" (`.Location` (`GameplayStatics.BreakHitResult` _outhit)) (`KismetMathLibrary.MakeRotFromZ` (`.Normal` (`GameplayStatics.BreakHitResult` _outhit)))) ; Spawn gun hit if not an enemy
        )))))

(event `Key|Two`
  (params (Key :type "Key Structure" :default "AnyKey"))
  ;[1 1 1] Debug (Cheat)
  (:`Pressed`
    (message `/Game/Blueprints/Interfaces/BPI_VRGameMode.SpawnPlayer` (`GameplayStatics.GetGameMode`) 2)))

(event `Key|Three`
  (params (Key :type "Key Structure" :default "AnyKey"))
  ;[1 1 1] Debug (Cheat)
  (:`Pressed`
    (message `/Game/Blueprints/Interfaces/BPI_VRGameMode.SpawnPlayer` (`GameplayStatics.GetGameMode`) 3)))

(event `Key|Four`
  (params (Key :type "Key Structure" :default "AnyKey"))
  ;[1 1 1] Debug (Cheat)
  (:`Pressed`
    (message `/Game/Blueprints/Interfaces/BPI_VRGameMode.SpawnPlayer` (`GameplayStatics.GetGameMode`) 4)))

(event `Key|Escape`
  (params (Key :type "Key Structure" :default "AnyKey"))
  (:`Pressed`
    (`KismetSystemLibrary.QuitGame` null "Quit")))

(fn `GetPlayerBodyLocation`
  (returns (Location :type "Vector Structure"))
  (bind (_returnvalue_x _returnvalue_y _returnvalue_z) (`KismetMathLibrary.BreakVector` (`SceneComponent.K2_GetComponentLocation` (`self.HMDCamera`))))
  (return (`KismetMathLibrary.MakeVector` _returnvalue_x _returnvalue_y (- _returnvalue_z 40.0))))

(fn `UserConstructionScript`)