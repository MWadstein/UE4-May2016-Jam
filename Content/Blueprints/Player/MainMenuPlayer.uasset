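; VR main menu player with motion controllers that starts the game from trigger presses; Escape quits.
; Each tick a trace from the teleport firing point tracks button targeting and toggles the MainMenuBP highlight on changes.
; Left trigger on a targeted button fades out and opens PersistentMap.
; Right trigger traces from the gun firing point, and any hit fades out and opens PersistentLevel.
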(event `self.ReceiveTick`
  (params (DeltaSeconds :type "Float (single-precision)"))
  (bind _teleportfiringpoint (`self.TeleportFiringPoint`))
  (bind _returnvalue (`SceneComponent.K2_GetComponentLocation` _teleportfiringpoint))
  ;[1 1 1] TeleportTrace
  (bind (_outhit _returnvalue_2) (`KismetSystemLibrary.LineTraceSingle` _returnvalue (+ _returnvalue (* (`KismetMathLibrary.GetForwardVector` (`SceneComponent.K2_GetComponentRotation` _teleportfiringpoint)) 1000.0)) "TraceTypeQuery3"))
  (if _returnvalue_2
    (set `self.HitActor` (`.HitActor` (`GameplayStatics.BreakHitResult` _outhit))) ; Safe Reference
  )
  (if (!= _returnvalue_2 (`self.ButtonTargetted`))
    (if (not (`self.ButtonTargetted`))
      (bind _output_get (set `self.ButtonTargetted` true))
      (`/Game/Blueprints/Helpers/MainMenuBP.ToggleColor` (cast `/Game/Blueprints/Helpers/MainMenuBP` (`self.HitActor`) :!pure true) _output_get)
      (else
        (bind _output_get_2 (set `self.ButtonTargetted` false))
        (`/Game/Blueprints/Helpers/MainMenuBP.ToggleColor` (cast `/Game/Blueprints/Helpers/MainMenuBP` (`self.HitActor`) :!pure true) _output_get_2)))))

(event `Key|MotionController_Left_Trigger`
  (params (Key :type "Key Structure" :default "AnyKey"))
  ;[1 1 1] Pull Left (Teleport) Trigger Event
  (:`Pressed`
    (if (`self.ButtonTargetted`)
      (`PlayerCameraManager.StartCameraFade` :`self` (`GameplayStatics.GetPlayerCameraManager` 0) :`FromAlpha` 0.0 :`ToAlpha` 1.0 :`Duration` 0.2 :`bHoldWhenFinished` true)
      (`KismetSystemLibrary.Delay` 1.0)
      (`GameplayStatics.OpenLevel` "PersistentMap"))))

(event `Key|MotionController_Right_Trigger`
  (params (Key :type "Key Structure" :default "AnyKey"))
  (bind _gunfiringpoint (`self.GunFiringPoint`))
  (bind _returnvalue (`SceneComponent.K2_GetComponentLocation` _gunfiringpoint))
  ;[1 1 1] Pull Right (Gun) Trigger Event
  (:`Pressed`
    (bind (_outhit _returnvalue_2) (`KismetSystemLibrary.LineTraceSingle` :`Start` _returnvalue :`End` (+ _returnvalue (* (`KismetMathLibrary.GetForwardVector` (`SceneComponent.K2_GetComponentRotation` _gunfiringpoint)) 1000.0)) :`TraceChannel` "TraceTypeQuery3" :`DrawDebugType` "ForOneFrame"))
    (if _returnvalue_2
      (`PlayerCameraManager.StartCameraFade` :`self` (`GameplayStatics.GetPlayerCameraManager` 0) :`FromAlpha` 0.0 :`ToAlpha` 1.0 :`Duration` 0.2 :`bHoldWhenFinished` true)
      (`KismetSystemLibrary.Delay` 1.0)
      (`GameplayStatics.OpenLevel` "PersistentLevel"))))

(event `Key|Escape`
  (params (Key :type "Key Structure" :default "AnyKey"))
  (:`Pressed`
    (`KismetSystemLibrary.QuitGame` null "Quit")))

(fn `GetPlayerBodyLocation`
  (returns (Location :type "Vector Structure"))
  (bind (_returnvalue_x _returnvalue_y _returnvalue_z) (`KismetMathLibrary.BreakVector` (`SceneComponent.K2_GetComponentLocation` (`self.HMDCamera`))))
  (return (`KismetMathLibrary.MakeVector` _returnvalue_x _returnvalue_y (- _returnvalue_z 40.0))))

(fn `UserConstructionScript`)