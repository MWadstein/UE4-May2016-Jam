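; Helper Blueprint that plays the game's intro dialog as a timed series of audio lines.
; The PlayTheIntroDialog event runs one linear chain of thirteen 2D sound plays, each followed by a hard-coded Delay that paces the conversation.
; Timing is independent of actual clip lengths, and the chain has no skip, interrupt or completion callback.
; The construction script is empty.
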(event `PlayTheIntroDialog`
  (`GameplayStatics.PlaySound2D` "/Game/Audio/1.1")
  (`KismetSystemLibrary.Delay` 3.0)
  (`GameplayStatics.PlaySound2D` "/Game/Audio/2.2")
  (`KismetSystemLibrary.Delay` 9.0)
  (`GameplayStatics.PlaySound2D` "/Game/Audio/3.3")
  (`KismetSystemLibrary.Delay` 1.0)
  (`GameplayStatics.PlaySound2D` "/Game/Audio/4.4")
  (`KismetSystemLibrary.Delay` 8.0)
  (`GameplayStatics.PlaySound2D` "/Game/Audio/5.5")
  (`KismetSystemLibrary.Delay` 1.5)
  (`GameplayStatics.PlaySound2D` "/Game/Audio/6.6")
  (`KismetSystemLibrary.Delay` 9.0)
  (`GameplayStatics.PlaySound2D` "/Game/Audio/7.7")
  (`KismetSystemLibrary.Delay` 3.0)
  (`GameplayStatics.PlaySound2D` "/Game/Audio/8.8")
  (`KismetSystemLibrary.Delay` 17.0)
  (`GameplayStatics.PlaySound2D` "/Game/Audio/9.9")
  (`KismetSystemLibrary.Delay` 4.0)
  (`GameplayStatics.PlaySound2D` "/Game/Audio/10.10")
  (`KismetSystemLibrary.Delay` 13.0)
  (`GameplayStatics.PlaySound2D` "/Game/Audio/11.11")
  (`KismetSystemLibrary.Delay` 16.0)
  (`GameplayStatics.PlaySound2D` "/Game/Audio/12.12")
  (`KismetSystemLibrary.Delay` 4.0)
  (`GameplayStatics.PlaySound2D` "/Game/Audio/13.13")
  (`KismetSystemLibrary.Delay` 17.0))

(fn `UserConstructionScript`)