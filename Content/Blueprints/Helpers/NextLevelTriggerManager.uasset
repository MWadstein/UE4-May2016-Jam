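; NextLevelTriggerManager gates progress by removing a designated actor once all target enemies are destroyed.
; A timer starts the first check after BeginPlay, then reschedules it while targets remain.
; Each check counts actors of ClassForClearTarget via IsDestroyed on an Enemy_Level3 cast and shows the remaining count on a TextWidget.
; At zero, it destroys ItemToRemoveWhenClear, clears the timer and destroys itself.
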(event `self.ReceiveBeginPlay`
  (bind _returnvalue (`KismetSystemLibrary.K2_SetTimer` null "CheckForCleared" 5.0))
  (set `self.TimerHandle` _returnvalue))

(event `CheckForCleared`
  (set `self.NumTargetsLeft` 0)
  (bind _outactors (`GameplayStatics.GetAllActorsOfClass` (`self.ClassForClearTarget`)))
  (for _array_element _outactors
    (if (not (`/Game/Blueprints/Enemies/Enemy_Parent.IsDestroyed` (cast `/Game/Blueprints/Enemies/Enemy_Level3` _array_element :!pure true)))
      (set `self.NumTargetsLeft` (+ (`self.NumTargetsLeft`) 1))))
  (if (<= (`self.NumTargetsLeft`) 0)
    (`self.K2_DestroyActor` (`self.ItemToRemoveWhenClear`))
    (`KismetSystemLibrary.K2_ClearTimerHandle` (`self.TimerHandle`))
    (`self.K2_DestroyActor`)
    (else
      (`self.SetWidgetText`)
      (bind _returnvalue (`KismetSystemLibrary.K2_SetTimer` null "CheckForCleared" 2.0))
      (set `self.TimerHandle` _returnvalue))))

(fn `SetWidgetText`
  (`/Game/Blueprints/Widgets/TextWidget.SetText` (cast `/Game/Blueprints/Widgets/TextWidget` (`WidgetComponent.GetUserWidgetObject` (`self.Widget`)) :!pure true) (`KismetTextLibrary.Conv_StringToText` (`KismetStringLibrary.Concat_StrStr` "Remaining: " (`KismetStringLibrary.Conv_IntToString` (`self.NumTargetsLeft`)))))
  (return))

(fn `UserConstructionScript`)