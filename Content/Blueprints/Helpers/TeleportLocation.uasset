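; TeleportLocation is a teleport destination marker that highlights when targeted.
; On BeginPlay it creates a dynamic material instance on its Cube.
; ToggleColor drives that material's Color parameter, showing green for a working location, red when IsBroken is set, and white when untargeted.
; GetTeleportLocation returns the Root world transform along with the IsBroken flag.
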(event `self.ReceiveBeginPlay`
  ;[1 1 1] Begin Play - Create our MID
  (bind _returnvalue (`PrimitiveComponent.CreateDynamicMaterialInstance` (`self.Cube`) 0 null))
  (set `self.MID` _returnvalue))

(event `/Game/Blueprints/Interfaces/BPI_TeleportLocation.ToggleColor`
  (params (Toggle :type Boolean))
  ;[1 1 1] Handle Toggling the Color if they target it
  (if (not (`self.IsBroken`))
    (`MaterialInstanceDynamic.SetVectorParameterValue` (`self.MID`) "Color" (select `bool` Toggle :`false` (struct :`R` 1.0 :`G` 1.0 :`B` 1.0 :`A` 1.0) :`true` (struct :`G` 1.0 :`A` 1.0) :!type "LinearColor Structure"))
    (else
      (`MaterialInstanceDynamic.SetVectorParameterValue` (`self.MID`) "Color" (select `bool` Toggle :`false` (struct :`R` 1.0 :`G` 1.0 :`B` 1.0 :`A` 1.0) :`true` (struct :`R` 1.0 :`A` 1.0) :!type "LinearColor Structure")))))

(fn `GetTeleportLocation`
  (returns (Transform :type "Transform Structure") (IsBroken :type Boolean))
  (return (`SceneComponent.K2_GetComponentToWorld` (`self.Root`)) (`self.IsBroken`)))

(fn `UserConstructionScript`)